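; BPKnight is a knight unit that taunts an enemy and attacks it when in range.
; Without a valid target, Tick sphere-overlaps for BPBaseEnemy pawns within TauntRange and claims the first result if untaunted, marking itself as the taunter.
; With a target, distance against AttackRange selects waiting or attacking.
; Those flags, both cleared while searching, are pushed to the ABP_Knight_SM animation instance every frame.
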(event EventTick
  (params (DeltaSeconds :type Float%20%28single-precision%29))
  (if (Utilities|IsValid (Variables|Default|GetTarget))
    (if (> (Math|Vector|Distance(Vector) (Transformation|GetActorLocation) (Transformation|GetActorLocation (Variables|Default|GetTarget))) (Variables|Default|GetAttackRange))
      (Variables|state|SetWaiting true)
      (Variables|State|SetAttacking false)
      (else
        (Variables|state|SetWaiting false)
        (Variables|State|SetAttacking true)))
    (else
      (bind (_outactors _returnvalue) (Collision|SphereOverlapActors (Transformation|GetActorLocation) (Variables|Default|GetTauntRange) (Utilities|Array|MakeArray "ObjectTypeQuery3") "/Game/Blueprints/BPBaseEnemy.BPBaseEnemy_C"))
      (if _returnvalue
        (bind _asbpbase_enemy (Utilities|Casting|CastToBPBaseEnemy (Utilities|Array|Get(acopy) _outactors)))
        (if (Class|BaseEnemy|GetIsTaunted _asbpbase_enemy)
          _
          (else
            (bind _output_get (Variables|Default|SetTarget (Utilities|Array|Get(acopy) _outactors)))
            (bind _asbpbase_enemy_2 (Utilities|Casting|CastToBPBaseEnemy _output_get))
            (Class|BaseEnemy|SetIsTaunted _asbpbase_enemy_2 true)
            (Class|BaseEnemy|SetTauntedby _asbpbase_enemy_2 self))))
      (Variables|state|SetWaiting false)
      (Variables|State|SetAttacking false)))
  (bind _asabp_knight_sm (Utilities|Casting|CastToABP_Knight_SM (Components|SkeletalMesh|GetAnimInstance (Variables|Character|GetMesh))))
  (Default|SetAttack _asabp_knight_sm (Variables|State|GetAttacking))
  (Default|SetWait _asabp_knight_sm (Variables|state|GetWaiting)))

(fn ConstructionScript
  (|CallParentFunction))