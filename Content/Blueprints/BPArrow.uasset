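; BPArrow is a homing arrow projectile that deals damage to a single assigned enemy target.
; Each tick it moves straight toward the Target at its Speed and rotates to face it with a fixed pitch offset, destroying itself if the Target is no longer valid.
; When its overlap sphere touches the Target, it calls Damage on it if it is a BPBaseEnemy, then destroys itself.
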(event OnComponentBeginOverlap(OverlapShere)
  (params (OverlappedComponent :type Primitive%20Component%20Object%20Reference) (OtherActor :type Actor%20Object%20Reference) (OtherComp :type Primitive%20Component%20Object%20Reference) (OtherBodyIndex :type Integer) (bFromSweep :type Boolean) (SweepResult :type Hit%20Result%20Structure%20%28by%20ref%29))
  (bind _target (Variables|Default|Gettarget))
  (if (== OtherActor _target)
    (bind _asbpbase_enemy (Utilities|Casting|CastToBPBaseEnemy _target)
      (:then
        (Class|BaseEnemy|Damage _asbpbase_enemy (Variables|Default|Getdamage)))
      (:CastFailed
        _))
    (Actor|DestroyActor)))

(event EventTick
  (params (DeltaSeconds :type Float%20%28single-precision%29))
  (bind _returnvalue (Transformation|GetActorLocation))
  (bind _target (Variables|Default|Gettarget))
  (bind _returnvalue_2 (Utilities|IsValid _target))
  (bind _returnvalue_3 (Transformation|GetActorLocation _target))
  (if _returnvalue_2
    (Transformation|AddActorWorldOffset (* (Math|Vector|Normalize (- _returnvalue_3 _returnvalue)) (Variables|Arrow|GetSpeed) DeltaSeconds))
    (if _returnvalue_2
      (Transformation|SetActorRotation (Math|Rotator|CombineRotators (Math|Rotator|FindLookatRotation _returnvalue _returnvalue_3) "0.000000,0.000000,-90.000000")))
    (else
      (Actor|DestroyActor))))

(fn ConstructionScript)