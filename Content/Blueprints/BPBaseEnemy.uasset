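; Base enemy Blueprint for the Vindolanda game mode, handling gold theft and kill reporting.
; ShowGold reveals the Gold component and deducts GoldSteal through the game mode's AddGold, while ReturnGold credits the same amount back.
; UpdateKilled notifies the game mode through EnemyKilled.
; The file only defines these events; none of them is triggered here.
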(event EventReturnGold
  (bind _asbpvindolanda_game_mode (Utilities|Casting|CastToBPVindolandaGameMode (Game|GetGameMode)))
  (Class|VindolandaGameMode|AddGold _asbpvindolanda_game_mode (Math|Float|Truncate (Variables|Default|GetgoldSteal))))

(event EventUpdateKilled
  (bind _asbpvindolanda_game_mode (Utilities|Casting|CastToBPVindolandaGameMode (Game|GetGameMode)))
  (Class|VindolandaGameMode|EnemyKilled _asbpvindolanda_game_mode))

(event EventShowGold
  (Rendering|SetVisibility (Variables|Default|GetGold) true false)
  (bind _asbpvindolanda_game_mode (Utilities|Casting|CastToBPVindolandaGameMode (Game|GetGameMode)))
  (Class|VindolandaGameMode|AddGold _asbpvindolanda_game_mode (Math|Float|Truncate (* (Variables|Default|GetgoldSteal) -1.0))))

(fn ConstructionScript)