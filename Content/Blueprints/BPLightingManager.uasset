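; Lighting manager that fades the scene between day and night.
; BeginPlay sets manual exposure on the post process; SetNight plays the Fade timeline forward for night or in reverse for day.
; Each update blends sun, moon and sky light intensities plus exposure compensation, and finishing recaptures the sky and commits IsNight.
; An older instant-switch chain in SetNight is left disconnected.
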(event EventBeginPlay
  (bind _postprocess (Variables|Default|GetPostProcess))
  (bind _postprocess_2 (Variables|Default|GetPostProcess))
  (bind _skylight (Variables|Default|GetSkyLight))
  (bind _structout (Utilities|Struct|SetmembersinPostProcessSettings (Variables|/Script/Engine.PostProcessVolume|GetSettings _postprocess) "AEM_Manual" (Variables|Default|GetDayExposureBias) false))
  (Variables|/Script/Engine.PostProcessVolume|SetSettings _postprocess _structout)
  (bind _alpha (Timeline|Fade SetNewTime)
    (:Update
      (Rendering|Components|Light|SetIntensity (Variables|/Script/Engine.SkyLight|GetLightComponent _skylight) (Math|Float|Lerp (Variables|Default|GetDaySkyIntensity) (Variables|Default|GetNightSkyIntensity) _alpha))
      (Rendering|Components|Light|SetIntensity (Variables|/Script/Engine.Light|GetLightComponent (Variables|Default|GetMoonLight)) (Math|Float|Lerp 0.0 (Variables|Default|GetNightMoonLux) _alpha))
      (Rendering|Components|Light|SetIntensity (Variables|/Script/Engine.Light|GetLightComponent (Variables|Default|GetSunLight)) (Math|Float|Lerp (Variables|Default|GetDaySunLux) 0.0 _alpha))
      (bind _structout_2 (Utilities|Struct|SetmembersinPostProcessSettings (Variables|/Script/Engine.PostProcessVolume|GetSettings _postprocess_2) (Math|Float|Lerp (Variables|Default|GetDayExposureBias) (Variables|Default|GetNightExposureBias) _alpha)))
      (Variables|/Script/Engine.PostProcessVolume|SetSettings _postprocess_2 _structout_2))
    (:Finished
      (Class|SkyLightComponent|RecaptureSky (Variables|/Script/Engine.SkyLight|GetLightComponent _skylight))
      (Variables|Default|SetisNight (Variables|Default|GetbTargetNight)))))

(fn ConstructionScript)

(fn SetNight
  (params (bNight :type Boolean))
  (bind _fade (Variables|Default|GetFade))
  (Variables|Default|SetbTargetNight bNight)
  (if bNight
    (Components|Timeline|PlayfromStart _fade)
    (else
      (Components|Timeline|ReversefromEnd _fade))))